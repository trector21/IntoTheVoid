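; Base Blueprint for a dual-bladed beam weapon that toggles on and off, with particle trails for the top and bottom blades.
; Toggle alternates sounds and timelines that animate the mesh material's Size parameter, setting trail visibility and the on/off state when each finishes.
; Trail events start and end socket-to-socket trails on both blades, playing a random swing sound only while on.
; The construction script pushes size, color, intensity and trail lifetime into materials and particles.
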(event `/Game/BeamWeapons/Blueprints/BPI_BeamWeapon.Toggle`
  (`/Engine/EditorBlueprintResources/StandardMacros.FlipFlop`
    (:`A`
      (`GameplayStatics.PlaySound2D` "/Game/BeamWeapons/Sounds/Toggle_Off_Cue.Toggle_Off_Cue" 1.0 1.0 0.0 null null)
      (bind (_direction _size) (`Timeline|Timeline_0_1` :!via `PlayFromStart`)
        (:`Update`
          (`MeshComponent.SetScalarParameterValueOnMaterials` (`self.Mesh`) "Size" _size))
        (:`Finished`
          (`SceneComponent.SetVisibility` (`self.Trails`) false false)
          (`SceneComponent.SetVisibility` (`self.Trails_Bottom`) false false)
          (set `self.SwordToggledOn?` false))))
    (:`B`
      (`GameplayStatics.PlaySound2D` "/Game/BeamWeapons/Sounds/Toggle_On_Cue.Toggle_On_Cue" 1.0 1.0 0.0 null null)
      (bind (_direction_2 _size_2) (`Timeline|Timeline_1_0` :!via `ReverseFromEnd`)
        (:`Update`
          (`MeshComponent.SetScalarParameterValueOnMaterials` (`self.Mesh`) "Size" _size_2))
        (:`Finished`
          (`SceneComponent.SetVisibility` (`self.Trails`) true false)
          (`SceneComponent.SetVisibility` (`self.Trails_Bottom`) true false)
          (set `self.SwordToggledOn?` true))))))

(event `/Game/BeamWeapons/Blueprints/BPI_BeamWeapon.Trails_On`
  (`ParticleSystemComponent.BeginTrails` (`self.Trails`) "Beginning" "End" "ETrailWidthMode_FromCentre" 1.0)
  (`ParticleSystemComponent.BeginTrails` (`self.Trails_Bottom`) "Beginning_2" "End_2" "ETrailWidthMode_FromCentre" 1.0)
  (if (`self.SwordToggledOn?`)
    (`GameplayStatics.PlaySound2D` (`|GetArrayItem` (`self.SwingSounds`) (`KismetMathLibrary.RandomIntegerInRange` 0 2)) 1.0 1.0 0.0 null null)))

(event `/Game/BeamWeapons/Blueprints/BPI_BeamWeapon.Trails_Off`
  (`|ExecutionSequence`
    (:`then_0`
      (`ParticleSystemComponent.EndTrails` (`self.Trails`)))
    (:`then_1`
      (`ParticleSystemComponent.EndTrails` (`self.Trails_Bottom`)))))

(fn `UserConstructionScript`
  (bind (_r _g _b) (`KismetMathLibrary.BreakColor` (`self.Color`)))
  (bind (_r_2 _g_2 _b_2) (`KismetMathLibrary.BreakColor` (`self.Color`)))
  (bind (_r_3 _g_3 _b_3) (`KismetMathLibrary.BreakColor` (`self.Color`)))
  (`MeshComponent.SetScalarParameterValueOnMaterials` (`self.Mesh`) "Size" (`self.Size`))
  (`MeshComponent.SetVectorParameterValueOnMaterials` (`self.Mesh`) "Color" (`KismetMathLibrary.Conv_LinearColorToVector` (`KismetMathLibrary.MakeColor` _r_2 _g_2 _b_2 (`self.ColorIntensity`))))
  (`FXSystemComponent.SetVectorParameter` (`self.Trails`) "ParticleColor" (`KismetMathLibrary.Conv_LinearColorToVector` (`KismetMathLibrary.MakeColor` _r _g _b (`self.ColorIntensity`))))
  (`FXSystemComponent.SetFloatParameter` (`self.Trails`) "TrailLifetime" (`self.TrailLifetime`))
  ;[1 1 1] To Control Bottom Trails
  (`FXSystemComponent.SetVectorParameter` (`self.Trails_Bottom`) "ParticleColor" (`KismetMathLibrary.Conv_LinearColorToVector` (`KismetMathLibrary.MakeColor` _r_3 _g_3 _b_3 (`self.ColorIntensity`))))
  (`FXSystemComponent.SetFloatParameter` (`self.Trails_Bottom`) "TrailLifetime" (`self.TrailLifetime`)))